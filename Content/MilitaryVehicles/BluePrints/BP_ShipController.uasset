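; BP_ShipController is a controller that exposes drivetrain telemetry from its controlled pawn, expecting a BP_TrackedVehicle despite the ship name.
; Getter functions cast the pawn and return left and right drive torque, engine torque, RPM, throttle and gearbox state.
; The gear getter returns placeholder values when the cast fails.
; Speed is the raw velocity length of any controlled pawn, with no cast or unit conversion.
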(fn ConstructionScript)

(fn GetDriveTLeft
  (bind _asbp_tracked_vehicle (Utilities|Casting|CastToBP_TrackedVehicle (Pawn|GetControlledPawn))
    (:then
      (LocalVariables|SetDriveT (Variables|/Game/MilitaryVehicles/BluePrints/BP_TrackedVehicle.BP_TrackedVehicle_C|GetDriveLeftTorque _asbp_tracked_vehicle)))
    (:CastFailed
      _))
  (return (LocalVariables|GetDriveT)))

(fn GetDriveTRight
  (bind _asbp_tracked_vehicle (Utilities|Casting|CastToBP_TrackedVehicle (Pawn|GetControlledPawn))
    (:then
      (LocalVariables|SetDriveT (Variables|/Game/MilitaryVehicles/BluePrints/BP_TrackedVehicle.BP_TrackedVehicle_C|GetDriveRightTorque _asbp_tracked_vehicle)))
    (:CastFailed
      _))
  (return (LocalVariables|GetDriveT)))

(fn GetEngineTorque
  (bind _asbp_tracked_vehicle (Utilities|Casting|CastToBP_TrackedVehicle (Pawn|GetControlledPawn))
    (:then
      (LocalVariables|SetEngineTorque (Variables|/Game/MilitaryVehicles/BluePrints/BP_TrackedVehicle.BP_TrackedVehicle_C|GetEngineTorque _asbp_tracked_vehicle)))
    (:CastFailed
      _))
  (return (LocalVariables|GetEngineTorque)))

(fn GetEnigineRPM
  (bind _asbp_tracked_vehicle (Utilities|Casting|CastToBP_TrackedVehicle (Pawn|GetControlledPawn))
    (:then
      (LocalVariables|SetRPM (Variables|/Game/MilitaryVehicles/BluePrints/BP_TrackedVehicle.BP_TrackedVehicle_C|GetEngineRPM _asbp_tracked_vehicle)))
    (:CastFailed
      _))
  (return (LocalVariables|GetRPM)))

(fn GetGear
  (bind _asbp_tracked_vehicle (Utilities|Casting|CastToBP_TrackedVehicle (Pawn|GetControlledPawn))
    (:then
      (bind (_gearnum _reversegear _automatic) (Default|GetGearBoxInfo _asbp_tracked_vehicle))
      (LocalVariables|SetGear _gearnum)
      (LocalVariables|SetReverse _reversegear)
      (LocalVariables|SetAutoGearB _automatic))
    (:CastFailed
      (LocalVariables|SetGear 10)
      (LocalVariables|SetReverse false)
      (LocalVariables|SetAutoGearB false)))
  (return (LocalVariables|GetGear) (LocalVariables|GetReverse) (LocalVariables|GetAutoGearB)))

(fn GetThrottle
  (bind _asbp_tracked_vehicle (Utilities|Casting|CastToBP_TrackedVehicle (Pawn|GetControlledPawn))
    (:then
      (LocalVariables|SetThrottlePrc (Variables|/Game/MilitaryVehicles/BluePrints/BP_TrackedVehicle.BP_TrackedVehicle_C|GetThrottle _asbp_tracked_vehicle)))
    (:CastFailed
      _))
  (return (LocalVariables|GetThrottlePrc)))

(fn GetVehicleSpeed
  (return (Math|Vector|VectorLength (Transformation|GetVelocity (Pawn|GetControlledPawn)))))