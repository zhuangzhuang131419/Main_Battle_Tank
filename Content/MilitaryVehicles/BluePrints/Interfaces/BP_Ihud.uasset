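; BP_Ihud is an interface of getters for military vehicle telemetry, apparently meant to feed a HUD.
; It exposes speed, engine RPM, engine torque, throttle and separate left and right DriveT values as single values.
; GetGear returns the gear index along with reverse and automatic gearbox flags.
; All functions here return only zero or false defaults and hold no logic.
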(fn GetVehicleSpeed
  (return 0.0))

(fn GetGear
  (return 0 false false))

(fn GetEnigineRPM
  (return 0.0))

(fn GetDriveTRight
  (return 0.0))

(fn GetDriveTLeft
  (return 0.0))

(fn GetThrottle
  (return 0.0))

(fn GetEngineTorque
  (return 0.0))