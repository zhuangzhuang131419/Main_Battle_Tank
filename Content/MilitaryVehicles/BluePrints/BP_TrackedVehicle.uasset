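; Base Blueprint for a drivable tracked military vehicle with auto/manual gearbox, orbit camera, rocket-firing cannon and turret HUD.
; Construction builds suspension, spline-placed instanced treads and track materials, leaving vehicle-specific handles and animation to child Blueprints.
; While awake, Tick updates throttle, engine and track velocities, animates treads, checks wheel collisions, then applies drive force and gathers friction torque per side.
; A looping timer updates the automatic gearbox.
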(event OnComponentHit(Body)
  (params (HitComponent :type Primitive%20Component%20Object%20Reference) (OtherActor :type Actor%20Object%20Reference) (OtherComp :type Primitive%20Component%20Object%20Reference) (NormalImpulse :type Vector :default "0, 0, 0") (Hit :type Hit%20Result%20Structure%20%28by%20ref%29))
  ;[1 1 1] Process collision
)

(event EventBeginPlay
  (Utilities|FlowControl|Sequence
    (:then_1
      (CallFunction|SetRemoveAutoGearBoxTimer true))
    (:then_2
      (CallFunction|TurretHud))))

(event EventPossessed
  (params (NewController :type Controller%20Object%20Reference))
  ;[1 1 1] AUDIO: Engine Start
  (Utilities|FlowControl|Delay 0.2)
  (Audio|PlaySoundatLocation "/Game/MilitaryVehicles/Sounds/Cue/start_Cue.start_Cue" (Transformation|GetActorLocation) "0, 0, 0" 1.0 1.0 0.0 0 0 0)
  (Audio|PlaySoundatLocation "/Game/MilitaryVehicles/Sounds/Cue/Engine_Loop.Engine_Loop" "0, 0, 0" "0, 0, 0" 1.0 1.0 0.0 0 0 0))

(event EventTick
  (params (DeltaSeconds :type Float%20%28single-precision%29))
  (bind _suspensionsinternalleft (Variables|Default|GetSuspensionsInternalLeft))
  (bind _suspensionsinternalright (Variables|Default|GetSuspensionsInternalRight))
  (bind _returnvalue (Class|TrackedVechile|PuttoSleep))
  (if (not _returnvalue)
    (Utilities|FlowControl|Sequence
      (:then_0
        (Class|TrackedVechile|UpdateThrottle)
        (Class|TrackedVechile|UpdateWheelsVelocity))
      (:then_1
        (CallFunction|AnimateWheels)
        (Class|TrackedVechile|AnimateTreadsMaterial)
        (CallFunction|AnimateTreadsSpline)
        (CallFunction|AnimateTreadsInstancedMesh))
      (:then_2
        (Class|TrackedVechile|UpdateAxlsVelocity)
        (Class|TrackedVechile|CalculateEngineandUpdateDrive))
      (:then_3
        (Utilities|FlowControl|Sequence
          (:then_0
            (for (_ _array_index) _suspensionsinternalright
              (Class|TrackedVechile|CheckWheelCollision _array_index _suspensionsinternalright "Right")))
          (:then_1
            (for (_ _array_index_2) _suspensionsinternalleft
              (Class|TrackedVechile|CheckWheelCollision _array_index_2 _suspensionsinternalleft "Left")))))
      (:then_4
        (Utilities|FlowControl|Sequence
          (:then_0
            (Class|TrackedVechile|CountFrictionContactPoint (Variables|Default|GetSuspensionsInternalRight)))
          (:then_1
            (Class|TrackedVechile|CountFrictionContactPoint (Variables|Default|GetSuspensionsInternalLeft)))))
      (:then_5
        (Utilities|FlowControl|Sequence
          (:then_0
            (bind (_totalfrictiontorqueside _totalrollingfrictiontoqueside) (Class|TrackedVechile|ApplyDriveForceandGetFrictionForceonSide (Variables|Default|GetSuspensionsInternalRight) (Variables|Default|GetDriveRightForce) (Variables|Default|GetTrackRightLinearVelocity)))
            (Variables|Default|SetTrackFrictionTorqueRight _totalfrictiontorqueside)
            (Variables|Default|SetTrackRollingFrictionTorqueRight _totalrollingfrictiontoqueside))
          (:then_1
            (bind (_totalfrictiontorqueside_2 _totalrollingfrictiontoqueside_2) (Class|TrackedVechile|ApplyDriveForceandGetFrictionForceonSide (Variables|Default|GetSuspensionsInternalLeft) (Variables|Default|GetDriveLeftForce) (Variables|Default|GetTrackLeftLinearVelocity)))
            (Variables|Default|SetTrackFrictionTorqueLeft _totalfrictiontorqueside_2)
            (Variables|Default|SetTrackRollingFrictionTorqueLeft _totalrollingfrictiontoqueside_2)
            (Variables|Default|SetTotalNumFrictionPoints 0)))))))

(event Input|ActionEvents|InputActionManualGearBox
  (params (Key :type Key%20Structure))
  ;[1 1 1] Switch between manual and auto gear box
  (:Pressed
    (Utilities|FlowControl|Delay 0.2)
    (Utilities|FlowControl|FlipFlop
      (:A
        (Variables|Default|SetAutoGearBox true)
        (Variables|Default|SetCurrentGear (+ (Variables|Default|GetNeutralGearIndex) 1)))
      (:B
        (Variables|Default|SetAutoGearBox false)))))

(event Input|ActionEvents|InputActionZoomIn
  (params (Key :type Key%20Structure))
  (bind _spring_arm (Variables|Default|GetSpring%20Arm))
  ;[1 1 1] Camera Control
  (:Pressed
    ;;[1 1 1] Draw spline tangents
    (Variables|/Script/Engine.SpringArmComponent|SetTargetArmLength _spring_arm (+ (Variables|/Script/Engine.SpringArmComponent|GetTargetArmLength _spring_arm) -25.0))))

(event Input|ActionEvents|InputActionZoomOut
  (params (Key :type Key%20Structure))
  (bind _spring_arm (Variables|Default|GetSpring%20Arm))
  ;[1 1 1] Camera Control
  (:Pressed
    (Variables|/Script/Engine.SpringArmComponent|SetTargetArmLength _spring_arm (+ (Variables|/Script/Engine.SpringArmComponent|GetTargetArmLength _spring_arm) 25.0))))

(event Input|ActionEvents|InputActionGearUp
  (params (Key :type Key%20Structure))
  ;[1 1 1] GearBox Manual Control
  (:Pressed
    (Utilities|FlowControl|Delay 0.2)
    (Class|TrackedVechile|ShiftGear 1)))

(event Input|ActionEvents|InputActionGearDown
  (params (Key :type Key%20Structure))
  ;[1 1 1] GearBox Manual Control
  (:Pressed
    (Utilities|FlowControl|Delay 0.2)
    (Class|TrackedVechile|ShiftGear -1)))

(event Input|ActionEvents|InputActionFire
  (params (Key :type Key%20Structure))
  ;[1 1 1] Main Gun
  (:Pressed
    (Game|SpawnActorfromClass "/Game/MilitaryVehicles/BluePrints/Rocket_projectile.Rocket_projectile_C" (Transformation|GetSocketTransform (Variables|Default|GetCannon) "Muzzle" "RTS_World") "AdjustIfPossibleButDontSpawnIfColliding" 0 0) ; Spawn projectile
    (Audio|PlaySoundatLocation "/Game/MilitaryVehicles/Sounds/Cue/Rocket.Rocket" (Transformation|GetActorLocation) "0, 0, 0" 1.5 1.0 0.0 0 0 0) ; Play firing sound
    (Effects|SpawnEmitterAttached "/Game/MilitaryVehicles/Particles/Rocket.Rocket" (Variables|Default|GetCannon) "Muzzle")))

(event Input|AxisEvents|InputAxisVehicleForwardBackward
  (params (AxisValue :type Float%20%28single-precision%29))
  ;[1 1 1] Vehicle Movement Controls
  (if (Variables|Default|GetAutoGearBox)
    (Class|TrackedVechile|GetThrottleInputforAutoHandling (stale Input|AxisEvents|InputAxisVehicleRightLeft AxisValue) AxisValue)
    (else
      (Variables|Default|SetWheelForwardCoefficient (Math|Float|Clamp(Float) AxisValue))
      (Variables|Default|SetBrakeRatio (* AxisValue (select (< AxisValue 0.0) -1.0 0.0)))))
  (if (or (!= (stale Input|AxisEvents|InputAxisVehicleRightLeft AxisValue) 0.0) (!= AxisValue 0.0))
    (Variables|Default|SetSleepMode false)
    (Variables|Default|SetSleepDelayTimer 0.0)))

(event Input|AxisEvents|InputAxisVehicleRightLeft
  (params (AxisValue :type Float%20%28single-precision%29))
  (bind _returnvalue (* AxisValue 1.0))
  (bind _returnvalue_2 (Math|Float|Absolute(Float) _returnvalue))
  ;[1 1 1] Vehicle Movement Controls
  (Variables|Default|SetWheelRightCoefficient (* _returnvalue_2 (select (< _returnvalue 0.0) 1.0 -1.0)))
  (Variables|Default|SetWheelLeftCoefficient (* _returnvalue_2 (select (< _returnvalue 0.0) -1.0 1.0)))
  (if (or (!= AxisValue 0.0) (!= (stale Input|AxisEvents|InputAxisVehicleForwardBackward AxisValue) 0.0))
    (Variables|Default|SetSleepMode false)
    (Variables|Default|SetSleepDelayTimer 0.0)))

(event Input|AxisEvents|InputAxisCameraVertical
  (params (AxisValue :type Float%20%28single-precision%29))
  ;[1 1 1] Camera Control
  (Transformation|AddLocalRotation (Variables|Default|GetSpring%20Arm) (Math|Rotator|MakeRotator 0.0 AxisValue 0.0) false false))

(event Input|AxisEvents|InputAxisCameraHorizontal
  (params (AxisValue :type Float%20%28single-precision%29))
  ;[1 1 1] Camera Control
  (Transformation|AddLocalRotation (Variables|Default|GetAzimuth%20Gimbal) (Math|Rotator|MakeRotator 0.0 0.0 AxisValue) false false))

(fn ConstructionScript
  (Utilities|FlowControl|Sequence
    (:then_0
      (Class|TrackedVechile|Initialise (Variables|Components|GetBody) (Variables|Components|GetCOM) (Variables|Components|GetTreadR) (Variables|Components|GetTreadL) (Variables|Components|GetWheelSweep) (Variables|Default|GetTurret) (Variables|Default|GetCannon)))
    (:then_1
      (Class|TrackedVechile|PreCalculateMomentOfInteria))
    (:then_2
      (Constructor|RegisterSuspensionHandles)
      (Constructor|ConstructSuspension))
    (:then_3
      (Class|TrackedVechile|VisualizeCenterOfMass))
    (:then_4
      (Constructor|CreateMaterialsforSimpleTracks))
    (:then_5
      (Constructor|BuildTrackSpline) ; Child blueprint will provide input parameters
    )
    (:then_6
      (Class|TrackedVechile|FindNeutralGearandSetStartingGear))))

(fn AnimateWheels
  ;[1 1 1] Dummy function, implement in child blueprints
  (return))

(fn AnimateTreadsSpline
  ;[1 1 1] Dummy function, implement in child blueprints
  (return))

(fn BuildTrackSpline
  (params (SplineR :type Spline%20Component%20Object%20Reference) (SplineL :type Spline%20Component%20Object%20Reference) (TreadsR :type Instanced%20Static%20Mesh%20Component%20Object%20Reference) (TreadsL :type Instanced%20Static%20Mesh%20Component%20Object%20Reference))
  (LocalVariables|SetSplineRLoc SplineR)
  (LocalVariables|SetSplineLLoc SplineL)
  (LocalVariables|SetTreadsRLoc TreadsR)
  (LocalVariables|SetTreadsLLoc TreadsL)
  (Variables|Default|SetTreadsLastIndexCPlusPlus (Math|Float|Truncate (- (Variables|Default|GetTreadsOnSide) 1.0)))
  (Spline|SetSplinePoints (LocalVariables|GetSplineRLoc) (Variables|Performance|GetSplineCoordinatesR) "Local" true)
  (Spline|SetSplinePoints (LocalVariables|GetSplineLLoc) (Variables|Performance|GetSplineCoordinatesL) "Local" true)
  (for (_array_element _array_index) (Variables|Performance|GetSplineTangents)
    (Spline|SetTangentatSplinePoint (LocalVariables|GetSplineRLoc) _array_index _array_element "Local" true)
    (Spline|SetTangentatSplinePoint (LocalVariables|GetSplineLLoc) _array_index _array_element "Local" true))
  (for _index (range 0 (Variables|Default|GetTreadsLastIndexCPlusPlus))
    (Components|InstancedStaticMesh|AddInstance (LocalVariables|GetTreadsRLoc) (Math|Transform|MakeTransform (Spline|GetLocationatDistanceAlongSpline (LocalVariables|GetSplineRLoc) (* _index (/ (Spline|GetSplineLength (LocalVariables|GetSplineRLoc)) 0.0)) "Local") (Math|Rotator|MakeRotator (Math|Float|SelectFloat 1.8e+02 (.roll (Spline|GetRotationatDistanceAlongSpline (LocalVariables|GetSplineRLoc) (* _index (/ (Spline|GetSplineLength (LocalVariables|GetSplineRLoc)) 0.0)) "Local")) (< (.y (Class|SplineComponent|GetRightVectoratDistanceAlongSpline (LocalVariables|GetSplineRLoc) (* _index (/ (Spline|GetSplineLength (LocalVariables|GetSplineRLoc)) 0.0)) "Local")) 0.0)) (.pitch (Spline|GetRotationatDistanceAlongSpline (LocalVariables|GetSplineRLoc) (* _index (/ (Spline|GetSplineLength (LocalVariables|GetSplineRLoc)) 0.0)) "Local")) (.yaw (Spline|GetRotationatDistanceAlongSpline (LocalVariables|GetSplineRLoc) (* _index (/ (Spline|GetSplineLength (LocalVariables|GetSplineRLoc)) 0.0)) "Local"))) (Math|Vector|MakeVector 1.0 1.0 1.0))))
  (for _index_2 (range 0 (Variables|Default|GetTreadsLastIndexCPlusPlus))
    (Components|InstancedStaticMesh|AddInstance (LocalVariables|GetTreadsLLoc) (Math|Transform|MakeTransform (Spline|GetLocationatDistanceAlongSpline (LocalVariables|GetSplineLLoc) (* _index_2 (/ (Spline|GetSplineLength (LocalVariables|GetSplineLLoc)) (Variables|Default|GetTreadsOnSide))) "Local") (Math|Rotator|MakeRotator (Math|Float|SelectFloat 1.8e+02 (.roll (Spline|GetRotationatDistanceAlongSpline (LocalVariables|GetSplineLLoc) (* _index_2 (/ (Spline|GetSplineLength (LocalVariables|GetSplineLLoc)) (Variables|Default|GetTreadsOnSide))) "Local")) (< (.y (Class|SplineComponent|GetRightVectoratDistanceAlongSpline (LocalVariables|GetSplineLLoc) (* _index_2 (/ (Spline|GetSplineLength (LocalVariables|GetSplineLLoc)) (Variables|Default|GetTreadsOnSide))) "Local")) 0.0)) (.pitch (Spline|GetRotationatDistanceAlongSpline (LocalVariables|GetSplineLLoc) (* _index_2 (/ (Spline|GetSplineLength (LocalVariables|GetSplineLLoc)) (Variables|Default|GetTreadsOnSide))) "Local")) (.yaw (Spline|GetRotationatDistanceAlongSpline (LocalVariables|GetSplineLLoc) (* _index_2 (/ (Spline|GetSplineLength (LocalVariables|GetSplineLLoc)) (Variables|Default|GetTreadsOnSide))) "Local"))) (Math|Vector|MakeVector 1.0 1.0 1.0))))
  (return false))

(fn ConstructSuspension
  (for (_array_element _array_index) (Variables|Internals|GetSuspHandleRight)
    (Utilities|Array|Add (Variables|Default|GetSuspensionsInternalRight) (Utilities|Struct|MakeSuspensionInternalProcessing (.location (Transformation|GetRelativeTransform _array_element)) (.rotation (Transformation|GetRelativeTransform _array_element)) (.maxlength (Utilities|Array|Get(acopy) (Variables|Default|GetSuspensionSetUpRight) _array_index)) (.collisionradius (Utilities|Array|Get(acopy) (Variables|Default|GetSuspensionSetUpRight) _array_index)) (.stiffnessforce (Utilities|Array|Get(acopy) (Variables|Default|GetSuspensionSetUpRight) _array_index)) (.dampingforce (Utilities|Array|Get(acopy) (Variables|Default|GetSuspensionSetUpRight) _array_index)) 0.0 "0.000000,0.000000,0.000000" "0.000000,0.000000,0.000000" "0.000000,0.000000,0.000000" false)))
  (for (_array_element_2 _array_index_2) (Variables|Internals|GetSuspHandleLeft)
    (Utilities|Array|Add (Variables|Default|GetSuspensionsInternalLeft) (Utilities|Struct|MakeSuspensionInternalProcessing (.location (Transformation|GetRelativeTransform _array_element_2)) (.rotation (Transformation|GetRelativeTransform _array_element_2)) (.maxlength (Utilities|Array|Get(acopy) (Variables|Default|GetSuspensionSetUpLeft) _array_index_2)) (.collisionradius (Utilities|Array|Get(acopy) (Variables|Default|GetSuspensionSetUpLeft) _array_index_2)) (.stiffnessforce (Utilities|Array|Get(acopy) (Variables|Default|GetSuspensionSetUpLeft) _array_index_2)) (.dampingforce (Utilities|Array|Get(acopy) (Variables|Default|GetSuspensionSetUpLeft) _array_index_2)) 0.0 "0.000000,0.000000,0.000000" "0.000000,0.000000,0.000000" "0.000000,0.000000,0.000000" false))))

(fn CreateMaterialsforSimpleTracks
  (Utilities|FlowControl|Sequence
    (:then_0
      (bind _returnvalue (Rendering|Material|CreateDynamicMaterialInstance "/Game/MilitaryVehicles/Materials/MI_Tread_Inst.MI_Tread_Inst" "None" :!class /Script/Engine.KismetMaterialLibrary))
      (Variables|Default|SetTreadMaterialRight _returnvalue)
      (bind _returnvalue_2 (Rendering|Material|CreateDynamicMaterialInstance "/Game/MilitaryVehicles/Materials/MI_Tread_Inst.MI_Tread_Inst" "None" :!class /Script/Engine.KismetMaterialLibrary))
      (Variables|Default|SetTreadMaterialLeft _returnvalue_2))
    (:then_1
      (Rendering|Material|SetMaterial (Variables|Components|GetTreadR) 0 (Variables|Default|GetTreadMaterialRight))
      (Rendering|Material|SetMaterial (Variables|Components|GetTreadL) 0 (Variables|Default|GetTreadMaterialLeft)))))

(fn RegisterSuspensionHandles
  ;[1 1 1] Dummy function, implement in child blueprints
  (return))

(fn AnimateTreadsInstancedMesh
  (params (SplineR :type Spline%20Component%20Object%20Reference) (SplineL :type Spline%20Component%20Object%20Reference) (TreadsR :type Instanced%20Static%20Mesh%20Component%20Object%20Reference) (TreadsL :type Instanced%20Static%20Mesh%20Component%20Object%20Reference))
  (Utilities|FlowControl|Sequence
    (:then_0
      (Class|TrackedVechile|AnimateTreadsInstancedMeshCPlusPlus SplineR TreadsR "Right"))
    (:then_1
      (Class|TrackedVechile|AnimateTreadsInstancedMeshCPlusPlus SplineL TreadsL "Left"))))

(fn SetRemoveAutoGearBoxTimer
  (params (SetTimer? :type Boolean))
  (if SetTimer?
    (bind _returnvalue (Utilities|Time|SetTimerbyFunctionName 0 "UpdateAutoGearBox" 0.5 true))
    (Variables|Internals|SetAutoGearBoxTimerHandle _returnvalue)
    (else
      (Utilities|Time|ClearandInvalidateTimerbyHandle (Variables|Internals|GetAutoGearBoxTimerHandle)))))

(fn TurretHud
  ;[1 1 1] Turret Hud widgets
  (bind _returnvalue (UserInterface|CreateWidget "/Game/MilitaryVehicles/BluePrints/UMG/BP_turretHuD.BP_turretHuD_C" (Game|GetPlayerController 0)))
  (UserInterface|Viewport|AddtoViewport _returnvalue 0)
  (return))

(fn HudWIdget
  ;[1 1 1] Turret Hud widgets
  (bind _returnvalue (UserInterface|CreateWidget "/Game/MilitaryVehicles/BluePrints/UMG/BP_VehicleHUD.BP_VehicleHUD_C" (Game|GetPlayerController 0)))
  (UserInterface|Viewport|AddtoViewport _returnvalue 0)
  (return))

(fn GetBackCoupler
  (return 0))

(fn GetFrontCoupler
  (return 0))